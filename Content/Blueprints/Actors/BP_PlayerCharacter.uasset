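; BP_PlayerCharacter is the player character Blueprint, handling body mesh setup and the visible weapon model.
; BeginPlay branches on local control, though both branches set the same Liam skeletal mesh.
; SwapWeaponMeshes sets the Weapon static mesh from a weapon ID: Glock 17, Machine Gun or Scar.
; Tick runs a debug-drawn visibility line trace along the weapon's negative forward axis, leaving the result unused.
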(event `self.ReceiveBeginPlay`
  (if (`self.IsLocallyControlled`)
    (`SkinnedMeshComponent.SetSkinnedAssetAndUpdate` (`self.Mesh`) "/Game/Characters_Mixamo/Liam/Liam.Liam" true)
    (else
      (`SkinnedMeshComponent.SetSkinnedAssetAndUpdate` (`self.Mesh`) "/Game/Characters_Mixamo/Liam/Liam.Liam" true))))

(event `self.ReceiveTick`
  (params (DeltaSeconds :type "Float (single-precision)"))
  (bind _weapon (`self.Weapon`))
  (bind _returnvalue (`SceneComponent.K2_GetComponentLocation` _weapon))
  (`KismetSystemLibrary.LineTraceSingle` :`Start` _returnvalue :`End` (+ _returnvalue (* (`SceneComponent.GetForwardVector` _weapon) -500.0)) :`TraceChannel` "TraceTypeQuery1" :`DrawDebugType` "ForOneFrame"))

(event `self.SwapWeaponMeshes`
  (params (newSelectedWeaponID :type "EWeaponID Enum" :default "AK47"))
  (switch `EWeaponID` newSelectedWeaponID
    (:`GLOCK17`
      (`StaticMeshComponent.SetStaticMesh` (`self.Weapon`) "/Game/THROW_AWAY/WeaponsPreview/Glock_17.Glock_17"))
    (:`MACHINE_GUN`
      (`StaticMeshComponent.SetStaticMesh` (`self.Weapon`) "/Game/THROW_AWAY/Models/Weapons/MG42/mg42_0.mg42_0"))
    (:`SCAR`
      (`StaticMeshComponent.SetStaticMesh` (`self.Weapon`) "/Game/THROW_AWAY/WeaponsPreview/Scar.Scar"))))

(fn `UserConstructionScript`)