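; Lobby HUD that creates the lobby widget on BeginPlay and supplies button styles for weapon slot buttons.
; GetWeaponButtonStyleByID switches on a weapon ID to one getter per weapon or item, plus an empty slot.
; Each getter builds a button style from that item's image, shared brush size and normal/hovered tints, with pressed reusing hovered.
; MP5 is the exception, using the normal tint for all states.
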(event `self.ReceiveBeginPlay`
  (bind _returnvalue (`|CreateWidget` "/Game/Blueprints/UMG/Lobby/UMG_HUD_Lobby.UMG_HUD_Lobby_C"))
  (bind _output_get (set `self.Widget_Lobby` _returnvalue))
  (`UserWidget.AddToViewport` _output_get 0))

(fn `GetButtonStyle_AK47`
  (returns (NewParam :type "ButtonStyle Structure"))
  (bind _slatebrush (make `SlateBrush` (`self.WeaponsSlotButtonSlateBrushSize`) (struct) (`self.WeaponsSlotButtonSlateColorHovered`) "/Game/THROW_AWAY/DEBUG/Lobby_Weapon_Slots_Placeholders/WSL_AK47.WSL_AK47"))
  (return (make `ButtonStyle` (make `SlateBrush` (`self.WeaponsSlotButtonSlateBrushSize`) (struct) (`self.WeaponsSlotButtonSlateColorNormal`) "/Game/THROW_AWAY/DEBUG/Lobby_Weapon_Slots_Placeholders/WSL_AK47.WSL_AK47") _slatebrush _slatebrush)))

(fn `GetButtonStyle_DesertEagle`
  (returns (NewParam :type "ButtonStyle Structure"))
  (bind _slatebrush (make `SlateBrush` (`self.WeaponsSlotButtonSlateBrushSize`) (struct) (`self.WeaponsSlotButtonSlateColorHovered`) "/Game/THROW_AWAY/DEBUG/Lobby_Weapon_Slots_Placeholders/WSL_DesertEagleGold.WSL_DesertEagleGold"))
  (return (make `ButtonStyle` (make `SlateBrush` (`self.WeaponsSlotButtonSlateBrushSize`) (struct) (`self.WeaponsSlotButtonSlateColorNormal`) "/Game/THROW_AWAY/DEBUG/Lobby_Weapon_Slots_Placeholders/WSL_DesertEagleGold.WSL_DesertEagleGold") _slatebrush _slatebrush)))

(fn `GetButtonStyle_EmptySlot`
  (returns (NewParam :type "ButtonStyle Structure"))
  (bind _slatebrush (make `SlateBrush` (`self.WeaponsSlotButtonSlateBrushSize`) (struct) (`self.WeaponsSlotButtonSlateColorHovered`) "/Game/THROW_AWAY/DEBUG/Lobby_Weapon_Slots_Placeholders/WSL_EmptySlot.WSL_EmptySlot"))
  (return (make `ButtonStyle` (make `SlateBrush` (`self.WeaponsSlotButtonSlateBrushSize`) (struct) (`self.WeaponsSlotButtonSlateColorNormal`) "/Game/THROW_AWAY/DEBUG/Lobby_Weapon_Slots_Placeholders/WSL_EmptySlot.WSL_EmptySlot") _slatebrush _slatebrush)))

(fn `GetButtonStyle_Glock`
  (returns (NewParam :type "ButtonStyle Structure"))
  (bind _slatebrush (make `SlateBrush` (`self.WeaponsSlotButtonSlateBrushSize`) (struct) (`self.WeaponsSlotButtonSlateColorHovered`) "/Game/THROW_AWAY/DEBUG/Lobby_Weapon_Slots_Placeholders/WSL_Glock17.WSL_Glock17"))
  (return (make `ButtonStyle` (make `SlateBrush` (`self.WeaponsSlotButtonSlateBrushSize`) (struct) (`self.WeaponsSlotButtonSlateColorNormal`) "/Game/THROW_AWAY/DEBUG/Lobby_Weapon_Slots_Placeholders/WSL_Glock17.WSL_Glock17") _slatebrush _slatebrush)))

(fn `GetButtonStyle_Grenade`
  (returns (NewParam :type "ButtonStyle Structure"))
  (bind _slatebrush (make `SlateBrush` (`self.WeaponsSlotButtonSlateBrushSize`) (struct) (`self.WeaponsSlotButtonSlateColorHovered`) "/Game/THROW_AWAY/DEBUG/Lobby_Weapon_Slots_Placeholders/WSL_Grenade.WSL_Grenade"))
  (return (make `ButtonStyle` (make `SlateBrush` (`self.WeaponsSlotButtonSlateBrushSize`) (struct) (`self.WeaponsSlotButtonSlateColorNormal`) "/Game/THROW_AWAY/DEBUG/Lobby_Weapon_Slots_Placeholders/WSL_Grenade.WSL_Grenade") _slatebrush _slatebrush)))

(fn `GetButtonStyle_HandPounch`
  (returns (NewParam :type "ButtonStyle Structure"))
  (bind _slatebrush (make `SlateBrush` (`self.WeaponsSlotButtonSlateBrushSize`) (struct) (`self.WeaponsSlotButtonSlateColorHovered`) "/Game/THROW_AWAY/DEBUG/Lobby_Weapon_Slots_Placeholders/WSL_HandsPounching.WSL_HandsPounching"))
  (return (make `ButtonStyle` (make `SlateBrush` (`self.WeaponsSlotButtonSlateBrushSize`) (struct) (`self.WeaponsSlotButtonSlateColorNormal`) "/Game/THROW_AWAY/DEBUG/Lobby_Weapon_Slots_Placeholders/WSL_HandsPounching.WSL_HandsPounching") _slatebrush _slatebrush)))

(fn `GetButtonStyle_L96`
  (returns (NewParam :type "ButtonStyle Structure"))
  (bind _slatebrush (make `SlateBrush` (`self.WeaponsSlotButtonSlateBrushSize`) (struct) (`self.WeaponsSlotButtonSlateColorHovered`) "/Game/THROW_AWAY/DEBUG/Lobby_Weapon_Slots_Placeholders/WSL_L96_Rifle.WSL_L96_Rifle"))
  (return (make `ButtonStyle` (make `SlateBrush` (`self.WeaponsSlotButtonSlateBrushSize`) (struct) (`self.WeaponsSlotButtonSlateColorNormal`) "/Game/THROW_AWAY/DEBUG/Lobby_Weapon_Slots_Placeholders/WSL_L96_Rifle.WSL_L96_Rifle") _slatebrush _slatebrush)))

(fn `GetButtonStyle_M16`
  (returns (NewParam :type "ButtonStyle Structure"))
  (bind _slatebrush (make `SlateBrush` (`self.WeaponsSlotButtonSlateBrushSize`) (struct) (`self.WeaponsSlotButtonSlateColorHovered`) "/Game/THROW_AWAY/DEBUG/Lobby_Weapon_Slots_Placeholders/WSL_M16.WSL_M16"))
  (return (make `ButtonStyle` (make `SlateBrush` (`self.WeaponsSlotButtonSlateBrushSize`) (struct) (`self.WeaponsSlotButtonSlateColorNormal`) "/Game/THROW_AWAY/DEBUG/Lobby_Weapon_Slots_Placeholders/WSL_M16.WSL_M16") _slatebrush _slatebrush)))

(fn `GetButtonStyle_Machete`
  (returns (NewParam :type "ButtonStyle Structure"))
  (bind _slatebrush (make `SlateBrush` (`self.WeaponsSlotButtonSlateBrushSize`) (struct) (`self.WeaponsSlotButtonSlateColorHovered`) "/Game/THROW_AWAY/DEBUG/Lobby_Weapon_Slots_Placeholders/WSL_Machete.WSL_Machete"))
  (return (make `ButtonStyle` (make `SlateBrush` (`self.WeaponsSlotButtonSlateBrushSize`) (struct) (`self.WeaponsSlotButtonSlateColorNormal`) "/Game/THROW_AWAY/DEBUG/Lobby_Weapon_Slots_Placeholders/WSL_Machete.WSL_Machete") _slatebrush _slatebrush)))

(fn `GetButtonStyle_MachineGun`
  (returns (NewParam :type "ButtonStyle Structure"))
  (bind _slatebrush (make `SlateBrush` (`self.WeaponsSlotButtonSlateBrushSize`) (struct) (`self.WeaponsSlotButtonSlateColorHovered`) "/Game/THROW_AWAY/DEBUG/Lobby_Weapon_Slots_Placeholders/WSL_MachineGun.WSL_MachineGun"))
  (return (make `ButtonStyle` (make `SlateBrush` (`self.WeaponsSlotButtonSlateBrushSize`) (struct) (`self.WeaponsSlotButtonSlateColorNormal`) "/Game/THROW_AWAY/DEBUG/Lobby_Weapon_Slots_Placeholders/WSL_MachineGun.WSL_MachineGun") _slatebrush _slatebrush)))

(fn `GetButtonStyle_MedicKit`
  (returns (NewParam :type "ButtonStyle Structure"))
  (bind _slatebrush (make `SlateBrush` (`self.WeaponsSlotButtonSlateBrushSize`) (struct) (`self.WeaponsSlotButtonSlateColorHovered`) "/Game/THROW_AWAY/DEBUG/Lobby_Weapon_Slots_Placeholders/WSL_MedicBox.WSL_MedicBox"))
  (return (make `ButtonStyle` (make `SlateBrush` (`self.WeaponsSlotButtonSlateBrushSize`) (struct) (`self.WeaponsSlotButtonSlateColorNormal`) "/Game/THROW_AWAY/DEBUG/Lobby_Weapon_Slots_Placeholders/WSL_MedicBox.WSL_MedicBox") _slatebrush _slatebrush)))

(fn `GetButtonStyle_Minigun`
  (returns (NewParam :type "ButtonStyle Structure"))
  (bind _slatebrush (make `SlateBrush` (`self.WeaponsSlotButtonSlateBrushSize`) (struct) (`self.WeaponsSlotButtonSlateColorHovered`) "/Game/THROW_AWAY/DEBUG/Lobby_Weapon_Slots_Placeholders/WSL_MiniGun.WSL_MiniGun"))
  (return (make `ButtonStyle` (make `SlateBrush` (`self.WeaponsSlotButtonSlateBrushSize`) (struct) (`self.WeaponsSlotButtonSlateColorNormal`) "/Game/THROW_AWAY/DEBUG/Lobby_Weapon_Slots_Placeholders/WSL_MiniGun.WSL_MiniGun") _slatebrush _slatebrush)))

(fn `GetButtonStyle_MP5`
  (returns (NewParam :type "ButtonStyle Structure"))
  (bind _slatebrush (make `SlateBrush` (`self.WeaponsSlotButtonSlateBrushSize`) (struct) (`self.WeaponsSlotButtonSlateColorNormal`) "/Game/THROW_AWAY/DEBUG/Lobby_Weapon_Slots_Placeholders/WSL_MP5.WSL_MP5"))
  (return (make `ButtonStyle` (make `SlateBrush` (`self.WeaponsSlotButtonSlateBrushSize`) (struct) (`self.WeaponsSlotButtonSlateColorNormal`) "/Game/THROW_AWAY/DEBUG/Lobby_Weapon_Slots_Placeholders/WSL_MP5.WSL_MP5") _slatebrush _slatebrush)))

(fn `GetButtonStyle_P60`
  (returns (NewParam :type "ButtonStyle Structure"))
  (bind _slatebrush (make `SlateBrush` (`self.WeaponsSlotButtonSlateBrushSize`) (struct) (`self.WeaponsSlotButtonSlateColorHovered`) "/Game/THROW_AWAY/DEBUG/Lobby_Weapon_Slots_Placeholders/WSL_P60.WSL_P60"))
  (return (make `ButtonStyle` (make `SlateBrush` (`self.WeaponsSlotButtonSlateBrushSize`) (struct) (`self.WeaponsSlotButtonSlateColorNormal`) "/Game/THROW_AWAY/DEBUG/Lobby_Weapon_Slots_Placeholders/WSL_P60.WSL_P60") _slatebrush _slatebrush)))

(fn `GetButtonStyle_R8`
  (returns (NewParam :type "ButtonStyle Structure"))
  (bind _slatebrush (make `SlateBrush` (`self.WeaponsSlotButtonSlateBrushSize`) (struct) (`self.WeaponsSlotButtonSlateColorHovered`) "/Game/THROW_AWAY/DEBUG/Lobby_Weapon_Slots_Placeholders/WSL_R8_Rifle.WSL_R8_Rifle"))
  (return (make `ButtonStyle` (make `SlateBrush` (`self.WeaponsSlotButtonSlateBrushSize`) (struct) (`self.WeaponsSlotButtonSlateColorNormal`) "/Game/THROW_AWAY/DEBUG/Lobby_Weapon_Slots_Placeholders/WSL_R8_Rifle.WSL_R8_Rifle") _slatebrush _slatebrush)))

(fn `GetButtonStyle_Revolver`
  (returns (NewParam :type "ButtonStyle Structure"))
  (bind _slatebrush (make `SlateBrush` (`self.WeaponsSlotButtonSlateBrushSize`) (struct) (`self.WeaponsSlotButtonSlateColorHovered`) "/Game/THROW_AWAY/DEBUG/Lobby_Weapon_Slots_Placeholders/WSL_Revolver.WSL_Revolver"))
  (return (make `ButtonStyle` (make `SlateBrush` (`self.WeaponsSlotButtonSlateBrushSize`) (struct) (`self.WeaponsSlotButtonSlateColorNormal`) "/Game/THROW_AWAY/DEBUG/Lobby_Weapon_Slots_Placeholders/WSL_Revolver.WSL_Revolver") _slatebrush _slatebrush)))

(fn `GetButtonStyle_RPG`
  (returns (NewParam :type "ButtonStyle Structure"))
  (bind _slatebrush (make `SlateBrush` (`self.WeaponsSlotButtonSlateBrushSize`) (struct) (`self.WeaponsSlotButtonSlateColorHovered`) "/Game/THROW_AWAY/DEBUG/Lobby_Weapon_Slots_Placeholders/WSL_RPG.WSL_RPG"))
  (return (make `ButtonStyle` (make `SlateBrush` (`self.WeaponsSlotButtonSlateBrushSize`) (struct) (`self.WeaponsSlotButtonSlateColorNormal`) "/Game/THROW_AWAY/DEBUG/Lobby_Weapon_Slots_Placeholders/WSL_RPG.WSL_RPG") _slatebrush _slatebrush)))

(fn `GetButtonStyle_Scar`
  (returns (NewParam :type "ButtonStyle Structure"))
  (bind _slatebrush (make `SlateBrush` (`self.WeaponsSlotButtonSlateBrushSize`) (struct) (`self.WeaponsSlotButtonSlateColorHovered`) "/Game/THROW_AWAY/DEBUG/Lobby_Weapon_Slots_Placeholders/WSL_Scar.WSL_Scar"))
  (return (make `ButtonStyle` (make `SlateBrush` (`self.WeaponsSlotButtonSlateBrushSize`) (struct) (`self.WeaponsSlotButtonSlateColorNormal`) "/Game/THROW_AWAY/DEBUG/Lobby_Weapon_Slots_Placeholders/WSL_Scar.WSL_Scar") _slatebrush _slatebrush)))

(fn `GetButtonStyle_Spanner`
  (returns (NewParam :type "ButtonStyle Structure"))
  (bind _slatebrush (make `SlateBrush` (`self.WeaponsSlotButtonSlateBrushSize`) (struct) (`self.WeaponsSlotButtonSlateColorHovered`) "/Game/THROW_AWAY/DEBUG/Lobby_Weapon_Slots_Placeholders/WSL_Spanner.WSL_Spanner"))
  (return (make `ButtonStyle` (make `SlateBrush` (`self.WeaponsSlotButtonSlateBrushSize`) (struct) (`self.WeaponsSlotButtonSlateColorNormal`) "/Game/THROW_AWAY/DEBUG/Lobby_Weapon_Slots_Placeholders/WSL_Spanner.WSL_Spanner") _slatebrush _slatebrush)))

(fn `GetButtonStyle_Stinger`
  (returns (NewParam :type "ButtonStyle Structure"))
  (bind _slatebrush (make `SlateBrush` (`self.WeaponsSlotButtonSlateBrushSize`) (struct) (`self.WeaponsSlotButtonSlateColorHovered`) "/Game/THROW_AWAY/DEBUG/Lobby_Weapon_Slots_Placeholders/WSL_Stinger.WSL_Stinger"))
  (return (make `ButtonStyle` (make `SlateBrush` (`self.WeaponsSlotButtonSlateBrushSize`) (struct) (`self.WeaponsSlotButtonSlateColorNormal`) "/Game/THROW_AWAY/DEBUG/Lobby_Weapon_Slots_Placeholders/WSL_Stinger.WSL_Stinger") _slatebrush _slatebrush)))

(fn `GetButtonStyly_AmmoBox`
  (returns (NewParam :type "ButtonStyle Structure"))
  (bind _slatebrush (make `SlateBrush` (`self.WeaponsSlotButtonSlateBrushSize`) (struct) (`self.WeaponsSlotButtonSlateColorHovered`) "/Game/THROW_AWAY/DEBUG/Lobby_Weapon_Slots_Placeholders/WSL_AmmoBox.WSL_AmmoBox"))
  (return (make `ButtonStyle` (make `SlateBrush` (`self.WeaponsSlotButtonSlateBrushSize`) (struct) (`self.WeaponsSlotButtonSlateColorNormal`) "/Game/THROW_AWAY/DEBUG/Lobby_Weapon_Slots_Placeholders/WSL_AmmoBox.WSL_AmmoBox") _slatebrush _slatebrush)))

(fn `GetWeaponButtonStyleByID`
  (params (`Weapon ID` :type "EWeaponID Enum" :default "AK47"))
  (returns (`New Button Style` :type "ButtonStyle Structure"))
  (switch `EWeaponID` `Weapon ID`
    (:`AK47`
      (bind _newparam (`self.GetButtonStyle_AK47`))
      (return _newparam))
    (:`AMMO_BOX`
      (bind _newparam_2 (`self.GetButtonStyly_AmmoBox`))
      (return _newparam_2))
    (:`DESERT_EAGLE`
      (bind _newparam_3 (`self.GetButtonStyle_DesertEagle`))
      (return _newparam_3))
    (:`GLOCK17`
      (bind _newparam_4 (`self.GetButtonStyle_Glock`))
      (return _newparam_4))
    (:`GRENADE`
      (bind _newparam_5 (`self.GetButtonStyle_Grenade`))
      (return _newparam_5))
    (:`HAND_POUNCH`
      (bind _newparam_6 (`self.GetButtonStyle_HandPounch`))
      (return _newparam_6))
    (:`L96`
      (bind _newparam_7 (`self.GetButtonStyle_L96`))
      (return _newparam_7))
    (:`M16`
      (bind _newparam_8 (`self.GetButtonStyle_M16`))
      (return _newparam_8))
    (:`MACHETE`
      (bind _newparam_9 (`self.GetButtonStyle_Machete`))
      (return _newparam_9))
    (:`MACHINE_GUN`
      (bind _newparam_10 (`self.GetButtonStyle_MachineGun`))
      (return _newparam_10))
    (:`MEDIC_BOX`
      (bind _newparam_11 (`self.GetButtonStyle_MedicKit`))
      (return _newparam_11))
    (:`MINIGUN`
      (bind _newparam_12 (`self.GetButtonStyle_Minigun`))
      (return _newparam_12))
    (:`MP5`
      (bind _newparam_13 (`self.GetButtonStyle_MP5`))
      (return _newparam_13))
    (:`P60`
      (bind _newparam_14 (`self.GetButtonStyle_P60`))
      (return _newparam_14))
    (:`R8`
      (bind _newparam_15 (`self.GetButtonStyle_R8`))
      (return _newparam_15))
    (:`REVOLVER`
      (bind _newparam_16 (`self.GetButtonStyle_Revolver`))
      (return _newparam_16))
    (:`RPG`
      (bind _newparam_17 (`self.GetButtonStyle_RPG`))
      (return _newparam_17))
    (:`SCAR`
      (bind _newparam_18 (`self.GetButtonStyle_Scar`))
      (return _newparam_18))
    (:`SPANNER`
      (bind _newparam_19 (`self.GetButtonStyle_Spanner`))
      (return _newparam_19))
    (:`STINGER`
      (bind _newparam_20 (`self.GetButtonStyle_Stinger`))
      (return _newparam_20))
    (:`NO_WEAPON`
      (bind _newparam_21 (`self.GetButtonStyle_EmptySlot`))
      (return _newparam_21))))

(fn `UserConstructionScript`)